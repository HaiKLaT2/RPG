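; Generic melee enemy AI character that the player can fight or stealth-assassinate from behind.
; The behavior tree calls Attack to run a two-montage sword combo, with input buffered during swings.
; Damage interrupts the combo, plays a random hit montage, launches the enemy along the player's facing and ragdolls it when BPCPlayerStats reports death.
; An overlap radius reveals the assassination prompt, while prompt, health bar and investigation icon face the camera every Tick.
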(event OnComponentBeginOverlap(AssasinationRadius)
  (params (OverlappedComponent :type Primitive%20Component%20Object%20Reference) (OtherActor :type Actor%20Object%20Reference) (OtherComp :type Primitive%20Component%20Object%20Reference) (OtherBodyIndex :type Integer) (bFromSweep :type Boolean) (SweepResult :type Hit%20Result%20Structure%20%28by%20ref%29))
  ;[1 1 1] Visibility of Widget
  (Utilities|Casting|CastToBP_ThirdPersonCharacter OtherActor)
  (Rendering|SetVisibility (Variables|Default|GetAssassinateWidget) true false))

(event OnComponentEndOverlap(AssasinationRadius)
  (params (OverlappedComponent :type Primitive%20Component%20Object%20Reference) (OtherActor :type Actor%20Object%20Reference) (OtherComp :type Primitive%20Component%20Object%20Reference) (OtherBodyIndex :type Integer))
  ;[1 1 1] Visibility of Widget
  (Utilities|Casting|CastToBP_ThirdPersonCharacter OtherActor)
  (Rendering|SetVisibility (Variables|Default|GetAssassinateWidget) false false))

(event Custom|SwordAttack
  ;[1 1 1] Combo System
  ;;[1 1 1] Sworld Attack
  (if (Variables|Default|Getis%20Attacking)
    (Variables|Default|Setsave%20Attack true)
    (else
      (Variables|Default|Setis%20Attacking true)
      (switch int (Variables|Default|GetAttack%20INDEX)
        (:0
          (CallFunction|Attack1))
        (:1
          (CallFunction|Attack2))))))

(event Custom|Sword%20Attack%20Combo
  ;[1 1 1] Combo System
  ;;[1 1 1] Combo Continue
  (if (Variables|Default|Getsave%20Attack)
    (Variables|Default|Setsave%20Attack false)
    (switch int (Variables|Default|GetAttack%20INDEX)
      (:0
        (CallFunction|Attack1))
      (:1
        (CallFunction|Attack2)))
    (else
      (CallFunction|StopSwordCombo))))

(event Custom|Sword%20Attack%20Combo%20Call%20From%20BT
  ;[1 1 1] Combo System
  ;;[1 1 1] Attack Input
  (if (Variables|Default|Getcan%20Attack?)
    (CallFunction|SwordAttack)))

(event Custom|Stop%20Sword%20Combo
  ;[1 1 1] Combo System
  ;;[1 1 1] Stop Combo/Attack
  (Variables|Default|Setis%20Attacking false)
  (Variables|Default|SetAttack%20INDEX 0))

(event Custom|Attack3
  ;[1 1 1] Combo System
  ;;[1 1 1] Attack3
  (Utilities|FlowControl|DoOnce false :!label _label
    (:Completed
      (Utilities|FlowControl|Delay 0.1)
      (Animation|Montage|PlayMontage (Variables|Character|GetMesh) "/Game/Characters/RPG_Character/Animations/SwordAttacks/Attack3_Montage.Attack3_Montage"
        (:then
          (Variables|Default|SetAttack%20INDEX 4)
          (goto _label Reset))))))

(event Custom|Attack1
  ;[1 1 1] Combo System
  ;;[1 1 1] Attack1
  (Utilities|FlowControl|DoOnce false :!label _label
    (:Completed
      (Utilities|FlowControl|Delay 0.1)
      (Animation|Montage|PlayMontage (Variables|Character|GetMesh) "/Game/Characters/RPG_Character/Animations/SwordAttacks/Attack1_Montage.Attack1_Montage" (Variables|Default|GetAttack%20Anim%20Speed)
        (:then
          (Variables|Default|SetAttack%20INDEX 1)
          (goto _label Reset))))))

(event Custom|Investigation%20Icon
  (bind _investigation_icon (Variables|Default|GetInvestigation%20Icon))
  ;[1 1 1] Combo System
  (Utilities|FlowControl|FlipFlop
    (:A
      (Rendering|SetVisibility _investigation_icon true false))
    (:B
      (Rendering|SetVisibility _investigation_icon false false))))

(event Custom|Attack2
  ;[1 1 1] Combo System
  ;;[1 1 1] Attack2
  (Utilities|FlowControl|DoOnce false :!label _label
    (:Completed
      (Utilities|FlowControl|Delay 0.1)
      (Animation|Montage|PlayMontage (Variables|Character|GetMesh) "/Game/Characters/RPG_Character/Animations/SwordAttacks/Attack2_Montage.Attack2_Montage" (Variables|Default|GetAttack%20Anim%20Speed)
        (:then
          (Variables|Default|SetAttack%20INDEX 2)
          (goto _label Reset))))))

(event Custom|AttackKIck
  ;[1 1 1] Combo System
  ;;[1 1 1] Attack Kick ( NOT in USE)
  (Utilities|FlowControl|DoOnce false :!label _label
    (:Completed
      (Utilities|FlowControl|Delay 0.1)
      (Animation|Montage|PlayMontage (Variables|Character|GetMesh) "/Game/Characters/RPG_Character/Animations/SwordAttacks/Kick_Montage.Kick_Montage"
        (:then
          (Variables|Default|SetAttack%20INDEX 3)
          (goto _label Reset))))))

(event Custom|RagDoll
  ;[1 1 1] RagDoll
  (Utilities|FlowControl|Sequence
    (:then_0
      (Utilities|FlowControl|Delay 2.5)
      (Physics|SetSimulatePhysics (Variables|Character|GetMesh) true))
    (:then_1
      (Utilities|FlowControl|Delay 1.5)
      (Audio|PlaySoundatLocation "/Game/Audio/Grunts-Hit/SC_Death.SC_Death" (Transformation|GetActorLocation) "0, 0, 0" 1.0 1.0 0.0 0 0 0 0))))

(event Collision|EventActorBeginOverlap
  (params (OtherActor :type Actor%20Object%20Reference)))

(event EventTick
  (params (DeltaSeconds :type Float%20%28single-precision%29))
  ;[1 1 1] Rotation of widget
  (Transformation|SetWorldRotation (Variables|Default|GetAssassinateWidget) (Math|Rotator|FindLookatRotation (Transformation|GetWorldLocation (Variables|Default|GetAssassinateWidget)) (Transformation|GetWorldLocation (Variables|/Script/Engine.PlayerCameraManager|GetTransformComponent (Game|GetPlayerCameraManager 0)))) false false))

(event Game|Damage|EventAnyDamage
  (params (Damage :type Float%20%28single-precision%29) (DamageType :type Damage%20Type%20Object%20Reference) (InstigatedBy :type Controller%20Object%20Reference) (DamageCauser :type Actor%20Object%20Reference))
  ;[1 1 1] Recive a hit
  (CallFunction|StopSwordCombo)
  (Animation|PlayAnimMontage (Utilities|Array|Get(acopy) (Variables|Default|GethitAnim) (Math|Random|RandomIntegerinRange 0 (- (Utilities|Array|Length (Variables|Default|GethitAnim)) 1))) 1.0 "None")
  (bind _asbp_third_person_character (Utilities|Casting|CastToBP_ThirdPersonCharacter (Game|GetPlayerCharacter 0)))
  (Character|LaunchCharacter (* (Math|Vector|GetForwardVector (Transformation|GetActorRotation _asbp_third_person_character)) 7e+02) false false)
  (Audio|PlaySoundatLocation "/Game/Audio/Grunts-Hit/SC_Death.SC_Death" (Math|Rotator|GetRotationXVector (Transformation|GetActorRotation)) "0, 0, 0" 1.0 1.0 0.0 0 0 0 0)
  (bind _ispalyer_dead (Default|DecreaseHealth (Variables|Default|GetBPC_PlayerStats) Damage))
  (if _ispalyer_dead
    (Physics|SetSimulatePhysics (Variables|Character|GetMesh) true)
    (Audio|PlaySoundatLocation "/Game/Audio/Grunts-Hit/SC_Death.SC_Death" (Transformation|GetActorLocation) "0, 0, 0" 1.0 1.0 0.0 0 0 0 0)
    (Rendering|SetVisibility (Variables|Default|GetHeath%20Bar%20Widget) false false)))

(event EventBeginPlay
  (bind _aswb_dummy (Utilities|Casting|CastToWB_Dummy (UserInterface|GetWidget (Variables|Default|GetHeath%20Bar%20Widget))))
  (Variables|Default|SetHealth%20bar%20UI _aswb_dummy))

(fn ConstructionScript)

(fn StealthBackAssasin
  (Animation|PlayAnimMontage "/Game/Characters/RPG_Character/Animations/Assassinations/Paired_Knife_Stealth_KidneyAndNeck_Vic_Montage.Paired_Knife_Stealth_KidneyAndNeck_Vic_Montage" 1.0 "None")
  (CallFunction|RagDoll)
  (Rendering|SetVisibility (Variables|Default|GetAssassinateWidget) false false)
  (return (Transformation|GetWorldLocation (Variables|Default|GetAssasinREF)) (Transformation|GetActorRotation)))

(fn Attack
  (CallFunction|SwordAttackComboCallfromBT)
  (return 0.4))