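; Generic boss AI controller that runs the boss behavior tree and manages an on-screen boss health bar.
; It starts BT_AI_BOSS on BeginPlay.
; Combat activation and deactivation events create and remove the WB_BOSS_Health_Bar widget.
; While the widget is valid, Tick polls Health over MaxHealth to set the bar's fill percent.
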(event Custom|Activate%20Boss%20Combat
  (bind _returnvalue (UserInterface|CreateWidget "/Game/UI/WB_BOSS_Health_Bar.WB_BOSS_Health_Bar_C"))
  (bind _output_get (Variables|Default|SetBossHealthBarWiddget _returnvalue))
  (UserInterface|Viewport|AddtoViewport _output_get 0))

(event Custom|Deactivate%20Boss%20Combat
  (Widget|RemovefromParent (Variables|Default|GetBossHealthBarWiddget))
  (Variables|Default|SetBossHealthBarWiddget 0))

(event EventBeginPlay
  (AI|RunBehaviorTree "/Game/AI/Boss/BT_AI_BOSS.BT_AI_BOSS"))

(event EventTick
  (params (DeltaSeconds :type Float%20%28single-precision%29))
  (bind _bosshealthbarwiddget (Variables|Default|GetBossHealthBarWiddget)
    (:then
      (Progress|SetPercent (Variables|/Game/UI/WB_BOSS_Health_Bar.WB_BOSS_Health_Bar_C|GetHealth_BAR _bosshealthbarwiddget) (/ (Variables|Default|GetHealth) (Variables|Default|GetMax%20Health))))
    (:else)))

(fn ConstructionScript
  (|CallParentFunction))