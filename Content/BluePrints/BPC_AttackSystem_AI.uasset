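; Melee attack component for BP_AI_Generic that plays sword combo montages and deals damage to actors tagged Damageable.
; SwordAttack buffers repeat requests; SwordAttackCombo continues by AttackINDEX or resets, with only Attack1 and Attack2 wired into the chain.
; A looping timer sweeps sphere traces along the blade, gated by a timed DoOnce, while SphereTrace handles single-point stab and kick hits.
; Hits apply damage, sound, blood and camera shake; debug traces remain visible.
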(event Custom|SwordAttack
  ;[1 1 1] Combo System
  ;;[1 1 1] Sworld Attack
  (if (Variables|Default|Getis%20Attacking)
    (Variables|Default|Setsave%20Attack true)
    (else
      (Variables|Default|Setis%20Attacking true)
      (switch int (Variables|Default|GetAttack%20INDEX)
        (:0
          (CallFunction|Attack1))
        (:1
          (CallFunction|Attack2))))))

(event Custom|Sword%20Attack%20Combo
  ;[1 1 1] Combo System
  ;;[1 1 1] Combo Continue
  (if (Variables|Default|Getsave%20Attack)
    (Variables|Default|Setsave%20Attack false)
    (switch int (Variables|Default|GetAttack%20INDEX)
      (:0
        (CallFunction|Attack1))
      (:1
        (CallFunction|Attack2)))
    (else
      (CallFunction|StopSwordCombo))))

(event Custom|Sphere%20Trace
  (bind _character_bp (Variables|Default|GetCharacter%20BP))
  (bind _sphere_trace_pos (Variables|/Game/AI/BP_AI_Generic.BP_AI_Generic_C|GetSphere%20Trace%20POS _character_bp))
  (bind _returnvalue (Transformation|GetWorldLocation _sphere_trace_pos))
  ;[1 1 1] Sphere Trace for Stab and  Kiick
  (bind (_outhit _returnvalue_2) (Collision|SphereTraceByChannel _returnvalue _returnvalue 12.0 "TraceTypeQuery1" false 0 "ForDuration" true "(R=0.000000,G=0.179911,B=1.000000,A=1.000000)" "(R=0.968855,G=0.000000,B=1.000000,A=1.000000)" 1.0))
  ;[1 1 1] Apply Damage by kick
  (if _returnvalue_2
    (if (Actor|ActorHasTag (.HitActor (Collision|BreakHitResult _outhit)) "Damageable")
      (Game|Damage|ApplyDamage (.HitActor (Collision|BreakHitResult _outhit)) 1e+01 0 0)
      (CallFunction|PlaySwordHitSound)
      (Effects|SpawnEmitteratLocation "/Game/FXs/Particles/Blood/P_Blood_Splat_Cone.P_Blood_Splat_Cone" (.Location (Collision|BreakHitResult _outhit)) (Math|Rotator|MakeRotfromXY (.Normal (Collision|BreakHitResult _outhit)) (.Normal (Collision|BreakHitResult _outhit))) "0.400000,0.400000,0.400000")
      (Camera|PlayWorldCameraShake "/Game/BluePrints/BP_CameraShakeHit.BP_CameraShakeHit_C" (.Location (Collision|BreakHitResult _outhit)) 0.0 2e+03))))

(event Custom|Play%20Sword%20Hit%20Sound
  ;[1 1 1] Play Sword hit Sound
  (Audio|PlaySoundatLocation "/Game/Audio/Sword_HIts/MS_Sword_Hit.MS_Sword_Hit" (Transformation|GetActorLocation (Components|GetOwner)) "0, 0, 0" 1.0 1.0 0.0 "/Game/Audio/Footsteps/RockStone/SA_Footsteps.SA_Footsteps" 0 0 0))

(event Custom|Stop%20Sword%20Combo
  ;[1 1 1] Combo System
  ;;[1 1 1] Stop Combo/Attack
  (Variables|Default|Setis%20Attacking false)
  (Variables|Default|SetAttack%20INDEX 0))

(event Custom|Attack3
  ;[1 1 1] Combo System
  ;;[1 1 1] Attack3
  (Utilities|FlowControl|DoOnce false :!label _label
    (:Completed
      (Utilities|FlowControl|Delay 0.1)
      (Animation|Montage|PlayMontage (Variables|Default|GetCharacter%20Mesh) "/Game/Characters/RPG_Character/Animations/SwordAttacks/Attack3_Montage.Attack3_Montage"
        (:then
          (Variables|Default|SetAttack%20INDEX 4)
          (goto _label Reset))))))

(event Custom|Attack1
  ;[1 1 1] Combo System
  ;;[1 1 1] Attack1
  (Utilities|FlowControl|DoOnce false :!label _label
    (:Completed
      (Utilities|FlowControl|Delay 0.1)
      (Animation|Montage|PlayMontage (Variables|Default|GetCharacter%20Mesh) "/Game/Characters/RPG_Character/Animations/SwordAttacks/Attack1_Montage.Attack1_Montage"
        (:then
          (Variables|Default|SetAttack%20INDEX 1)
          (goto _label Reset))))))

(event Custom|Sword%20Trace
  ;[1 1 1] Sword Trace
  (bind _returnvalue (Utilities|Time|SetTimerbyEvent (delegate Custom|Sword%20Trace%20Loop) 0.001 true))
  (Variables|Default|SetSword_Trace_Loop _returnvalue))

(event Custom|Attack2
  ;[1 1 1] Combo System
  ;;[1 1 1] Attack2
  (Utilities|FlowControl|DoOnce false :!label _label
    (:Completed
      (Utilities|FlowControl|Delay 0.1)
      (Animation|Montage|PlayMontage (Variables|Default|GetCharacter%20Mesh) "/Game/Characters/RPG_Character/Animations/SwordAttacks/Attack2_Montage.Attack2_Montage"
        (:then
          (Variables|Default|SetAttack%20INDEX 2)
          (goto _label Reset))))))

(event Custom|Sword%20Trace%20Loop
  ;[1 1 1] Sword Trace
  (bind (_outhit _returnvalue) (Collision|SphereTraceByChannel (Transformation|GetWorldLocation (Variables|/Game/AI/BP_AI_Generic.BP_AI_Generic_C|GetSword_top_Point (Variables|Default|GetCharacter%20BP))) (Transformation|GetWorldLocation (Variables|/Game/AI/BP_AI_Generic.BP_AI_Generic_C|GetSword_Bottom_Point1 (Variables|Default|GetCharacter%20BP))) 12.0 "TraceTypeQuery1" false 0 "ForDuration" true "(R=1.000000,G=0.000000,B=0.000000,A=1.000000)" "(R=0.000000,G=1.000000,B=0.000000,A=1.000000)" 1.0))
  ;[1 1 1] Apply Damage by sword
  (if _returnvalue
    (if (Actor|ActorHasTag (.HitActor (Collision|BreakHitResult _outhit)) "Damageable")
      (Utilities|FlowControl|DoOnce false :!label _label
        (:Completed
          (Game|Damage|ApplyDamage (.HitActor (Collision|BreakHitResult _outhit)) 1e+01 0 0)
          (CallFunction|PlaySwordHitSound)
          (Effects|SpawnEmitteratLocation "/Game/FXs/Particles/Blood/P_Blood_Splat_Cone.P_Blood_Splat_Cone" (.Location (Collision|BreakHitResult _outhit)) (Math|Rotator|MakeRotfromXY (.Normal (Collision|BreakHitResult _outhit)) (.Normal (Collision|BreakHitResult _outhit))) "0.400000,0.400000,0.400000")
          (Camera|PlayWorldCameraShake "/Game/BluePrints/BP_CameraShakeHit.BP_CameraShakeHit_C" (.Location (Collision|BreakHitResult _outhit)) 0.0 2e+03)
          (Utilities|FlowControl|Delay 0.5)
          (goto _label Reset))))))

(event Custom|AttackKIck
  ;[1 1 1] Combo System
  ;;[1 1 1] Attack Kick
  (Utilities|FlowControl|DoOnce false :!label _label
    (:Completed
      (Utilities|FlowControl|Delay 0.1)
      (Animation|Montage|PlayMontage (Variables|Default|GetCharacter%20Mesh) "/Game/Characters/RPG_Character/Animations/SwordAttacks/Kick_Montage.Kick_Montage"
        (:then
          (Variables|Default|SetAttack%20INDEX 3)
          (goto _label Reset))))))

(event Custom|Stop%20Sword%20Trace
  ;[1 1 1] Sword Trace
  (Utilities|Time|ClearandInvalidateTimerbyHandle (Variables|Default|GetSword_Trace_Loop)))

(event Input|EnhancedActionEvents|EnhancedInputActionIA_Attack
  (params (ActionValue :type Boolean) (ElapsedSeconds :type Float%20%28double-precision%29) (TriggeredSeconds :type Float%20%28double-precision%29) (InputAction :type Input%20Action%20Object%20Reference :default "/Game/ThirdPerson/Input/Actions/IA_Attack.IA_Attack"))
  ;[1 1 1] Combo System
  ;;[1 1 1] Attack Input
  (:Started
    (if (Variables|Default|Getcan%20Attack?)
      (CallFunction|SwordAttack))))

(event EventBeginPlay
  (bind _asbp_ai_generic (Utilities|Casting|CastToBP_AI_Generic (Components|GetOwner)))
  (bind _output_get (Variables|Default|SetCharacter%20BP _asbp_ai_generic))
  (Variables|Default|SetCharacter%20Mesh (Variables|/Script/Engine.Character|GetMesh _output_get)))