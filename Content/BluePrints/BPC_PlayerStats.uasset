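; Stats component that tracks health, stamina, XP and level for the player, training dummies and generic AI.
; BeginPlay casts the owner to set a character type, which selects the HUD or health-bar widget that health setup and damage update directly.
; Decrease functions report depletion, while stamina, increase and XP functions write only to the player HUD.
; Reaching max XP levels up, resetting XP, raising the threshold and playing a sound.
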(event EventBeginPlay
  (Utilities|FlowControl|DelayUntilNextTick)
  (bind _asbp_third_person_character (Utilities|Casting|CastToBP_ThirdPersonCharacter (Components|GetOwner))
    (:then
      (Variables|Default|SetPlayer%20Character _asbp_third_person_character)
      (Variables|Default|SetisPlayer true)
      (Progress|SetPercent (Variables|/Game/UI/WB_Hud.WB_Hud_C|GetStaminaBar (Variables|/Game/ThirdPerson/Blueprints/BP_ThirdPersonCharacter.BP_ThirdPersonCharacter_C|GetHUD%20Widget (Variables|Default|GetPlayer%20Character))) (/ (Variables|Stamina|GetCurrent%20Stamina) (Variables|Stamina|GetMax%20Stamina)))
      ;[1 1 1] Show Health and Stamina Before Gain it
      (Variables|Default|SetCharacter%20TYPE "NewEnumerator0"))
    (:CastFailed
      (bind _asbp_dummy (Utilities|Casting|CastToBP_Dummy (Components|GetOwner))
        (:then
          (Variables|Default|SetAs%20BP%20Dummy _asbp_dummy)
          (Variables|Default|SetisPlayer false)
          (Variables|Default|SetCharacter%20TYPE "NewEnumerator1"))
        (:CastFailed
          (bind _asbp_ai_generic (Utilities|Casting|CastToBP_AI_Generic (Components|GetOwner)))
          (Variables|Default|SetAs%20BP%20AI%20Generic _asbp_ai_generic)
          (Variables|Default|SetCharacter%20TYPE "NewEnumerator2")))))
  (Progress|SetPercent (Utilities|Select :Index (Variables|Default|GetCharacter%20TYPE) :NewEnumerator0 (Variables|/Game/UI/WB_Hud.WB_Hud_C|GetHealthBar (Variables|/Game/ThirdPerson/Blueprints/BP_ThirdPersonCharacter.BP_ThirdPersonCharacter_C|GetHUD%20Widget (Variables|Default|GetPlayer%20Character))) :NewEnumerator1 (Variables|/Game/UI/WB_Dummy.WB_Dummy_C|GetHealthBar (Variables|/Game/BluePrints/BP_Dummy.BP_Dummy_C|GetHealth%20bar%20UI (Variables|Default|GetAs%20BP%20Dummy))) :NewEnumerator2 (Variables|/Game/UI/WB_Dummy.WB_Dummy_C|GetHealthBar (Variables|/Game/AI/BP_AI_Generic.BP_AI_Generic_C|GetHealth%20bar%20UI (Variables|Default|GetAs%20BP%20AI%20Generic)))) (/ (Variables|Health|GetCurrent%20Health) (Variables|Health|GetMax%20Health)))
  (Rendering|Components|TextRender|SetText (Utilities|Select :Index (Variables|Default|GetCharacter%20TYPE) :NewEnumerator0 (Variables|/Game/UI/WB_Hud.WB_Hud_C|GetHealthText (Variables|/Game/ThirdPerson/Blueprints/BP_ThirdPersonCharacter.BP_ThirdPersonCharacter_C|GetHUD%20Widget (Variables|Default|GetPlayer%20Character))) :NewEnumerator1 (Variables|/Game/UI/WB_Dummy.WB_Dummy_C|GetHealthText (Variables|/Game/BluePrints/BP_Dummy.BP_Dummy_C|GetHealth%20bar%20UI (Variables|Default|GetAs%20BP%20Dummy))) :NewEnumerator2 (Variables|/Game/UI/WB_Dummy.WB_Dummy_C|GetHealthText (Variables|/Game/AI/BP_AI_Generic.BP_AI_Generic_C|GetHealth%20bar%20UI (Variables|Default|GetAs%20BP%20AI%20Generic)))) (Utilities|Text|ToText(Float) (Variables|Health|GetCurrent%20Health) "HalfToEven"))
  (if (Variables|Default|GetisPlayer)
    (Progress|SetPercent (Variables|/Game/UI/WB_Hud.WB_Hud_C|GetXPBar (Variables|/Game/ThirdPerson/Blueprints/BP_ThirdPersonCharacter.BP_ThirdPersonCharacter_C|GetHUD%20Widget (Variables|Default|GetPlayer%20Character))) (/ (Variables|XP|GetXP) (Variables|XP|GetMax%20XP)))
    (Class|Widget|SetToolTipText (Variables|/Game/UI/WB_Hud.WB_Hud_C|GetXPBar (Variables|/Game/ThirdPerson/Blueprints/BP_ThirdPersonCharacter.BP_ThirdPersonCharacter_C|GetHUD%20Widget (Variables|Default|GetPlayer%20Character))) (Utilities|Text|ToText(Float) (Variables|XP|GetXP) "HalfToEven"))
    (Class|Widget|SetToolTipText (Variables|/Game/UI/WB_Hud.WB_Hud_C|GetLVLtxt (Variables|/Game/ThirdPerson/Blueprints/BP_ThirdPersonCharacter.BP_ThirdPersonCharacter_C|GetHUD%20Widget (Variables|Default|GetPlayer%20Character))) (Utilities|Text|ToText(Integer) (Variables|XP|GetLevel)))))

(fn DecreaseHealth
  (params (Damage :type Float%20%28double-precision%29))
  (if (not (<= (Variables|Health|GetCurrent%20Health) 0.0))
    (bind _output_get (Variables|Health|SetCurrent%20Health (- (Variables|Health|GetCurrent%20Health) Damage)))
    (Progress|SetPercent (Utilities|Select :Index (Variables|Default|GetCharacter%20TYPE) :NewEnumerator0 (Variables|/Game/UI/WB_Hud.WB_Hud_C|GetHealthBar (Variables|/Game/ThirdPerson/Blueprints/BP_ThirdPersonCharacter.BP_ThirdPersonCharacter_C|GetHUD%20Widget (Variables|Default|GetPlayer%20Character))) :NewEnumerator1 (Variables|/Game/UI/WB_Dummy.WB_Dummy_C|GetHealthBar (Variables|/Game/BluePrints/BP_Dummy.BP_Dummy_C|GetHealth%20bar%20UI (Variables|Default|GetAs%20BP%20Dummy))) :NewEnumerator2 (Variables|/Game/UI/WB_Dummy.WB_Dummy_C|GetHealthBar (Variables|/Game/AI/BP_AI_Generic.BP_AI_Generic_C|GetHealth%20bar%20UI (Variables|Default|GetAs%20BP%20AI%20Generic)))) (/ _output_get (Variables|Health|GetMax%20Health)))
    (Rendering|Components|TextRender|SetText (Utilities|Select :Index (Variables|Default|GetCharacter%20TYPE) :NewEnumerator0 (Variables|/Game/UI/WB_Hud.WB_Hud_C|GetHealthText (Variables|/Game/ThirdPerson/Blueprints/BP_ThirdPersonCharacter.BP_ThirdPersonCharacter_C|GetHUD%20Widget (Variables|Default|GetPlayer%20Character))) :NewEnumerator1 (Variables|/Game/UI/WB_Dummy.WB_Dummy_C|GetHealthText (Variables|/Game/BluePrints/BP_Dummy.BP_Dummy_C|GetHealth%20bar%20UI (Variables|Default|GetAs%20BP%20Dummy))) :NewEnumerator2 (Variables|/Game/UI/WB_Dummy.WB_Dummy_C|GetHealthText (Variables|/Game/AI/BP_AI_Generic.BP_AI_Generic_C|GetHealth%20bar%20UI (Variables|Default|GetAs%20BP%20AI%20Generic)))) (Utilities|Text|ToText(Float) (Variables|Health|GetCurrent%20Health) "HalfToEven"))
    (if (<= (Variables|Health|GetCurrent%20Health) 0.0)
      _
      (else
        (return false))))
  (return true))

(fn IncreaseMaxHealth
  (params (Max%20Health%20Inc :type Float%20%28double-precision%29))
  (bind _player_character (Variables|Default|GetPlayer%20Character))
  (bind _hud_widget (Variables|/Game/ThirdPerson/Blueprints/BP_ThirdPersonCharacter.BP_ThirdPersonCharacter_C|GetHUD%20Widget _player_character))
  (Variables|Health|SetMax%20Health (+ (Variables|Health|GetCurrent%20Health) Max%20Health%20Inc))
  (Progress|SetPercent (Variables|/Game/UI/WB_Hud.WB_Hud_C|GetHealthBar _hud_widget) (/ (Variables|Health|GetCurrent%20Health) (Variables|Health|GetMax%20Health)))
  (Rendering|Components|TextRender|SetText (Variables|/Game/UI/WB_Hud.WB_Hud_C|GetHealthText _hud_widget) (Utilities|Text|ToText(Float) (Variables|Health|GetCurrent%20Health) "HalfToEven")))

(fn DecreaseStamina
  (params (B :type Float%20%28double-precision%29))
  (if (not (<= (Variables|Stamina|GetCurrent%20Stamina) 0.0))
    (bind _output_get (Variables|Stamina|SetCurrent%20Stamina (- (Variables|Stamina|GetCurrent%20Stamina) B)))
    (Progress|SetPercent (Variables|/Game/UI/WB_Hud.WB_Hud_C|GetStaminaBar (Variables|/Game/ThirdPerson/Blueprints/BP_ThirdPersonCharacter.BP_ThirdPersonCharacter_C|GetHUD%20Widget (Variables|Default|GetPlayer%20Character))) (/ _output_get (Variables|Stamina|GetMax%20Stamina)))
    (if (<= (Variables|Stamina|GetCurrent%20Stamina) 0.0)
      _
      (else
        (return false))))
  (return true))

(fn IncreasaeMaxStamina
  (params (Added%20Stamina :type Float%20%28double-precision%29))
  (bind _player_character (Variables|Default|GetPlayer%20Character))
  (bind _hud_widget (Variables|/Game/ThirdPerson/Blueprints/BP_ThirdPersonCharacter.BP_ThirdPersonCharacter_C|GetHUD%20Widget _player_character))
  (Variables|Stamina|SetMax%20Stamina (+ (Variables|Stamina|GetCurrent%20Stamina) Added%20Stamina))
  (Progress|SetPercent (Variables|/Game/UI/WB_Hud.WB_Hud_C|GetStaminaBar _hud_widget) (/ (Variables|Stamina|GetCurrent%20Stamina) (Variables|Stamina|GetMax%20Stamina)))
  (Rendering|Components|TextRender|SetText (Variables|/Game/UI/WB_Hud.WB_Hud_C|GetStaminaText _hud_widget) (Utilities|Text|ToText(Float) (Variables|Stamina|GetCurrent%20Stamina) "HalfToEven")))

(fn IncreaseHealth
  (params (Added%20Health :type Float%20%28double-precision%29))
  (bind _player_character (Variables|Default|GetPlayer%20Character))
  (bind _hud_widget (Variables|/Game/ThirdPerson/Blueprints/BP_ThirdPersonCharacter.BP_ThirdPersonCharacter_C|GetHUD%20Widget _player_character))
  (Variables|Health|SetCurrent%20Health (+ (Variables|Health|GetCurrent%20Health) Added%20Health))
  (if (> (Variables|Health|GetCurrent%20Health) (Variables|Health|GetMax%20Health))
    (Variables|Health|SetCurrent%20Health (Variables|Health|GetMax%20Health)))
  (Progress|SetPercent (Variables|/Game/UI/WB_Hud.WB_Hud_C|GetHealthBar _hud_widget) (/ (Variables|Health|GetCurrent%20Health) (Variables|Health|GetMax%20Health)))
  (Rendering|Components|TextRender|SetText (Variables|/Game/UI/WB_Hud.WB_Hud_C|GetHealthText _hud_widget) (Utilities|Text|ToText(Float) (Variables|Health|GetCurrent%20Health) "HalfToEven")))

(fn IncreaseStamina
  (params (Added%20to%20Current%20Stamina :type Float%20%28double-precision%29))
  (bind _player_character (Variables|Default|GetPlayer%20Character))
  (bind _hud_widget (Variables|/Game/ThirdPerson/Blueprints/BP_ThirdPersonCharacter.BP_ThirdPersonCharacter_C|GetHUD%20Widget _player_character))
  (Variables|Stamina|SetCurrent%20Stamina (+ (Variables|Stamina|GetCurrent%20Stamina) Added%20to%20Current%20Stamina))
  (if (> (Variables|Stamina|GetCurrent%20Stamina) (Variables|Stamina|GetMax%20Stamina))
    (Variables|Stamina|SetCurrent%20Stamina (Variables|Stamina|GetMax%20Stamina)))
  (Progress|SetPercent (Variables|/Game/UI/WB_Hud.WB_Hud_C|GetStaminaBar _hud_widget) (/ (Variables|Stamina|GetCurrent%20Stamina) (Variables|Stamina|GetMax%20Stamina)))
  (Rendering|Components|TextRender|SetText (Variables|/Game/UI/WB_Hud.WB_Hud_C|GetStaminaText _hud_widget) (Utilities|Text|ToText(Float) (Variables|Stamina|GetCurrent%20Stamina) "HalfToEven")))

(fn IncreaseXP
  (params (Added%20XP :type Float%20%28double-precision%29))
  (Variables|XP|SetXP (+ (Variables|XP|GetXP) Added%20XP))
  (if (>= (Variables|XP|GetXP) (Variables|XP|GetMax%20XP))
    (LVLandXP|IncreaseLVL 1))
  (Progress|SetPercent (Variables|/Game/UI/WB_Hud.WB_Hud_C|GetXPBar (Variables|/Game/ThirdPerson/Blueprints/BP_ThirdPersonCharacter.BP_ThirdPersonCharacter_C|GetHUD%20Widget (Variables|Default|GetPlayer%20Character))) (/ (Variables|XP|GetXP) (Variables|XP|GetMax%20XP)))
  (Rendering|Components|TextRender|SetText (Variables|/Game/UI/WB_Hud.WB_Hud_C|GetCurrentXP (Variables|/Game/ThirdPerson/Blueprints/BP_ThirdPersonCharacter.BP_ThirdPersonCharacter_C|GetHUD%20Widget (Variables|Default|GetPlayer%20Character))) (Utilities|Text|FormatText "{Current XP} / {Max XP}" (Variables|XP|GetXP) (Variables|XP|GetMax%20XP))))

(fn IncreaseLVL
  (params (Added%20LVL :type Integer))
  (Variables|XP|SetLevel (+ (Variables|XP|GetLevel) Added%20LVL))
  (Variables|XP|SetMax%20XP (+ (Variables|XP|GetMax%20XP) 1.5e+02))
  (Variables|XP|SetXP 0.0)
  (Rendering|Components|TextRender|SetText (Variables|/Game/UI/WB_Hud.WB_Hud_C|GetLVLtxt (Variables|/Game/ThirdPerson/Blueprints/BP_ThirdPersonCharacter.BP_ThirdPersonCharacter_C|GetHUD%20Widget (Variables|Default|GetPlayer%20Character))) (Utilities|Text|ToText(Integer) (Variables|XP|GetLevel)))
  (if (> (Variables|XP|GetLevel) 1)
    (Audio|PlaySound2D "/Game/Audio/UI/475889__epicsoundeffects__ese-whoosh-epic-level-up.475889__epicsoundeffects__ese-whoosh-epic-level-up" 1.0 1.0 0.0 0 0)))