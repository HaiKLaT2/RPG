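; BP_Dummy is a target character that the player can hit or stealth-assassinate from behind.
; Damage plays a random hit montage, launches it along the player's facing and lowers BPCPlayerStats health, ragdolling it on death.
; An overlap radius toggles the assassinate prompt, which rotates with the health bar to face the camera.
; StealthBackAssasin plays the victim montage, triggers delayed ragdoll and returns the attacker's alignment location and rotation.
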(event OnComponentBeginOverlap(AssasinationRadius)
  (params (OverlappedComponent :type Primitive%20Component%20Object%20Reference) (OtherActor :type Actor%20Object%20Reference) (OtherComp :type Primitive%20Component%20Object%20Reference) (OtherBodyIndex :type Integer) (bFromSweep :type Boolean) (SweepResult :type Hit%20Result%20Structure%20%28by%20ref%29))
  ;[1 1 1] Visibility of Widget
  (Utilities|Casting|CastToBP_ThirdPersonCharacter OtherActor)
  (Rendering|SetVisibility (Variables|Default|GetAssassinateWidget) true false))

(event OnComponentEndOverlap(AssasinationRadius)
  (params (OverlappedComponent :type Primitive%20Component%20Object%20Reference) (OtherActor :type Actor%20Object%20Reference) (OtherComp :type Primitive%20Component%20Object%20Reference) (OtherBodyIndex :type Integer))
  ;[1 1 1] Visibility of Widget
  (Utilities|Casting|CastToBP_ThirdPersonCharacter OtherActor)
  (Rendering|SetVisibility (Variables|Default|GetAssassinateWidget) false false))

(event Custom|RagDoll
  ;[1 1 1] RagDoll
  (Utilities|FlowControl|Sequence
    (:then_0
      (Utilities|FlowControl|Delay 2.5)
      (Physics|SetSimulatePhysics (Variables|Character|GetMesh) true))
    (:then_1
      (Utilities|FlowControl|Delay 1.5)
      (Audio|PlaySoundatLocation "/Game/Audio/Grunts-Hit/SC_Death.SC_Death" (Transformation|GetActorLocation) "0, 0, 0" 1.0 1.0 0.0 0 0 0 0))))

(event Collision|EventActorBeginOverlap
  (params (OtherActor :type Actor%20Object%20Reference)))

(event EventTick
  (params (DeltaSeconds :type Float%20%28single-precision%29))
  ;[1 1 1] Rotation of widget
  (Transformation|SetWorldRotation (Variables|Default|GetAssassinateWidget) (Math|Rotator|FindLookatRotation (Transformation|GetWorldLocation (Variables|Default|GetAssassinateWidget)) (Transformation|GetWorldLocation (Variables|/Script/Engine.PlayerCameraManager|GetTransformComponent (Game|GetPlayerCameraManager 0)))) false false))

(event Game|Damage|EventAnyDamage
  (params (Damage :type Float%20%28single-precision%29) (DamageType :type Damage%20Type%20Object%20Reference) (InstigatedBy :type Controller%20Object%20Reference) (DamageCauser :type Actor%20Object%20Reference))
  ;[1 1 1] Recive a hit
  (Animation|PlayAnimMontage (Utilities|Array|Get(acopy) (Variables|Default|GethitAnim) (Math|Random|RandomIntegerinRange 0 (- (Utilities|Array|Length (Variables|Default|GethitAnim)) 1))) 1.0 "None")
  (bind _asbp_third_person_character (Utilities|Casting|CastToBP_ThirdPersonCharacter (Game|GetPlayerCharacter 0)))
  (Character|LaunchCharacter (* (Math|Vector|GetForwardVector (Transformation|GetActorRotation _asbp_third_person_character)) 7e+02) false false)
  (Audio|PlaySoundatLocation "/Game/Audio/Grunts-Hit/SC_Death.SC_Death" (Math|Rotator|GetRotationXVector (Transformation|GetActorRotation)) "0, 0, 0" 1.0 1.0 0.0 0 0 0 0)
  (bind _ispalyer_dead (Default|DecreaseHealth (Variables|Default|GetBPC_PlayerStats) Damage))
  (if _ispalyer_dead
    (Physics|SetSimulatePhysics (Variables|Character|GetMesh) true)
    (Audio|PlaySoundatLocation "/Game/Audio/Grunts-Hit/SC_Death.SC_Death" (Transformation|GetActorLocation) "0, 0, 0" 1.0 1.0 0.0 0 0 0 0)
    (Rendering|SetVisibility (Variables|Default|GetHeath%20Bar%20Widget) false false)))

(event EventBeginPlay
  (bind _aswb_dummy (Utilities|Casting|CastToWB_Dummy (UserInterface|GetWidget (Variables|Default|GetHeath%20Bar%20Widget))))
  (Variables|Default|SetHealth%20bar%20UI _aswb_dummy))

(fn ConstructionScript)

(fn StealthBackAssasin
  (Animation|PlayAnimMontage "/Game/Characters/RPG_Character/Animations/Assassinations/Paired_Knife_Stealth_KidneyAndNeck_Vic_Montage.Paired_Knife_Stealth_KidneyAndNeck_Vic_Montage" 1.0 "None")
  (CallFunction|RagDoll)
  (Rendering|SetVisibility (Variables|Default|GetAssassinateWidget) false false)
  (return (Transformation|GetWorldLocation (Variables|Default|GetAssasinREF)) (Transformation|GetActorRotation)))